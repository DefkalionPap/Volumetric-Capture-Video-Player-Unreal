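; Blueprint that plays volumetric capture video as a flipbook of static meshes, one mesh per frame.
; BeginPlay counts the frames in the mesh array, then Tick accumulates delta time and swaps the Static Mesh component's mesh at the FPS interval.
; A loop check gates playback on the loaded flag, so the sequence either restarts or stops after the last frame, resuming if Loop is enabled.
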(event EventBeginPlay
  (|InitializeVariables)
  (Variables|Default|SetvideoLoaded true)
  (Variables|Default|SetfixedUpdate 1.0))

(event EventTick
  (params (DeltaSeconds :type Float%20%28single-precision%29))
  (|CheckforLoop)
  (Variables|Default|Settimer (+ (Variables|Default|Gettimer) DeltaSeconds))
  (Variables|Default|SetframeDuration (/ 1.0 (Math|Conversions|ToFloat(Integer) (Variables|Default|GetFPS))))
  (if (>= (Variables|Default|Gettimer) (Variables|Default|GetframeDuration))
    (|PlayVideo)
    (Variables|Default|SetrenderedFrames (+ (Variables|Default|GetrenderedFrames) 1))
    (Variables|Default|Settimer (- (Variables|Default|Gettimer) (Variables|Default|GetframeDuration)))
    (if (== (Variables|Default|GetrenderedFrames) (Variables|Default|GettotalFramesCount))
      (if (== (Variables|Default|Getloop) true)
        (Variables|Default|SetrenderedFrames 0)
        (else
          (Variables|Default|SetrenderedFrames 0)
          (Variables|Default|SetvideoLoaded false))))))

(fn ConstructionScript)