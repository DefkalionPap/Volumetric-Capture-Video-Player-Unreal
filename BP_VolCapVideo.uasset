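; BP_VolCapVideo is an actor that loads a sample Duck glTF from a hardcoded GitHub URL at runtime, apparently as a volumetric video test.
; BeginPlay starts the glTFRuntime URL load, whose callback applies each mesh, then each material, to the single Video mesh component.
; Each pass overwrites the last, so only the final mesh and slot-0 material remain.
; Both loops use the mesh count, and debug prints report progress.
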(event Custom|CustomEvent
  (params (Asset :type Gl%20TF%20Runtime%20Asset%20Object%20Reference))
  (bind _returnvalue (Class|GlTFRuntimeAsset|GetNumMeshes Asset))
  (bind _video (Variables|Default|GetVideo))
  (bind _returnvalue_2 (- _returnvalue 1))
  (for _index (range 0 _returnvalue_2)
    (bind _returnvalue_3 (Class|GlTFRuntimeAsset|LoadStaticMesh Asset _index))
    (Components|StaticMesh|SetStaticMesh _video _returnvalue_3))
  (Development|PrintText "First mesh loaded")
  (for _index_2 (range 0 _returnvalue_2)
    (bind _returnvalue_4 (Class|GlTFRuntimeAsset|LoadMaterial :self Asset :MaterialIndex _index_2))
    (Rendering|Material|SetMaterial _video 0 _returnvalue_4))
  (Development|PrintText "First material loaded")
  (Development|PrintString (Utilities|String|Append "Total Meshes: " (Utilities|String|ToString(Integer) _returnvalue_2))))

(event EventBeginPlay
  (bind _output_get (Variables|Default|SetfilePath "https://raw.githubusercontent.com/KhronosGroup/glTF-Sample-Models/master/2.0/Duck/glTF-Embedded/Duck.gltf"))
  (Class|GlTFRuntimeFunctionLibrary|GlTFLoadAssetfromUrl _output_get 0 (delegate Custom|CustomEvent)))

(event Collision|EventActorBeginOverlap
  (params (OtherActor :type Actor%20Object%20Reference)))

(event EventTick
  (params (DeltaSeconds :type Float%20%28single-precision%29)))

(fn ConstructionScript)